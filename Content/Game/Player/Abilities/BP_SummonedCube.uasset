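; Summoned cube for a player ability that, once dropped, can squish actors beneath it.
; DropCube enables physics and gravity on the mesh, swaps it to stone and sets a short lifespan.
; Overlapping actors that have an Ability System Component receive GE_Squished while the cube is falling.
; Tick tracks falling from Box's vertical velocity and plays a camera shake on upward rebound, scaled by squared actor scale.
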(event OnComponentBeginOverlap(Box)
  (params (OverlappedComponent :type Primitive%20Component%20Object%20Reference) (OtherActor :type Actor%20Object%20Reference) (OtherComp :type Primitive%20Component%20Object%20Reference) (OtherBodyIndex :type Integer) (bFromSweep :type Boolean) (SweepResult :type Hit%20Result%20Structure%20%28by%20ref%29))
  (bind _returnvalue (Ability|GetAbilitySystemComponent OtherActor))
  (Utilities|IsValid _returnvalue
    (:Is%20Valid
      (if (Variables|Default|GetIsFalling)
        (GameplayEffects|ApplyGameplayEffectToSelf :self _returnvalue :GameplayEffectClass "/Game/Game/Player/Abilities/GE_Squished.GE_Squished_C")))))

(event EventBeginPlay)

(event EventTick
  (params (DeltaSeconds :type Float%20%28single-precision%29))
  (bind _returnvalue (Physics|GetPhysicsLinearVelocity (Variables|Default|GetBox) "None"))
  (if (and (Variables|Default|GetIsFalling) (> (.z _returnvalue) 0.0))
    (Class|LegacyCameraShake|StartLegacyCameraShake (Game|GetPlayerCameraManager 0) "/Game/Game/Player/Abilities/legacyCubeShaake.legacyCubeShaake_C" (Math|Float|Square (.x (Transformation|GetActorScale3D))) "CameraLocal" "0, 0, 0")
    (else
      (Variables|Default|SetIsFalling (< (.z _returnvalue) -1e+02)))))

(fn ConstructionScript)

(fn DropCube
  (bind _cube (Variables|Default|GetCube))
  (Physics|SetSimulatePhysics _cube true)
  (Physics|SetEnableGravity _cube true)
  (Variables|Default|SetIsFalling true)
  (Actor|SetLifeSpan 5.0)
  (Rendering|Material|SetMaterial (Variables|Default|GetCube) 0 "/Game/StarterContent/Materials/M_Brick_Cut_Stone.M_Brick_Cut_Stone"))