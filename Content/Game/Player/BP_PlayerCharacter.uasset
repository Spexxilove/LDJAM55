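; Player character with cursor aiming and a GAS ability that summons a cube, grown while the input is held.
; On possession it creates the HUD, grants the ability and chains attribute listeners that update health, trigger game over and rescale growth rate and duration.
; Tick faces the cursor hit, grows and moves the cube there, and adjusts camera arm length to cube height.
; Input also drives movement, ability confirmation on release and the pause menu.
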(event Input|EnhancedActionEvents|EnhancedInputActionIA_Move
  (params (ActionValue :type Vector%202D%20Structure) (ElapsedSeconds :type Float%20%28double-precision%29) (TriggeredSeconds :type Float%20%28double-precision%29) (InputAction :type Input%20Action%20Object%20Reference :default "/Game/Game/Input/Actions/IA_Move.IA_Move"))
  ;[1 1 1] movement
  (Class|PawnMovementComponent|AddInputVector (Variables|Character|GetCharacterMovement) (Math|Vector|MakeVector (.x ActionValue) (.y ActionValue) 0.0) false))

(event Input|EnhancedActionEvents|EnhancedInputActionIA_Summon
  (params (ActionValue :type Boolean) (ElapsedSeconds :type Float%20%28double-precision%29) (TriggeredSeconds :type Float%20%28double-precision%29) (InputAction :type Input%20Action%20Object%20Reference :default "/Game/Game/Input/Actions/IA_Summon.IA_Summon"))
  (bind _abilitysystem (Variables|Default|GetAbilitySystem))
  ;[1 1 1] Summon Cube
  (:Started
    (bind _returnvalue (Abilities|TryActivateAbilitybyClass _abilitysystem "/Game/Game/Player/Abilities/GA_SummonCube.GA_SummonCube_C" true))
    (Variables|Default|SetisSummoning _returnvalue))
  (:Completed
    (if (Variables|Default|GetisSummoning)
      (Class|AbilitySystemComponent|InputConfirm _abilitysystem)
      (Variables|Default|SetisSummoning false))))

(event Input|EnhancedActionEvents|EnhancedInputActionIA_Pause
  (params (ActionValue :type Boolean) (ElapsedSeconds :type Float%20%28double-precision%29) (TriggeredSeconds :type Float%20%28double-precision%29) (InputAction :type Input%20Action%20Object%20Reference :default "/Game/Game/Input/Actions/IA_Pause.IA_Pause"))
  (bind _returnvalue (UserInterface|CreateWidget "/Game/Game/UI/PauseMenu/WBP_PauseMenu.WBP_PauseMenu_C"))
  (UserInterface|Viewport|AddtoViewport _returnvalue 0))

(event EventPossessed
  (params (NewController :type Controller%20Object%20Reference))
  ;[1 1 1] HUD Setup
  (bind _asbp_player_controller (Utilities|Casting|CastToBP_PlayerController NewController))
  (bind _returnvalue (UserInterface|CreateWidget "/Game/Game/UI/HUD/WBP_HUD.WBP_HUD_C" _asbp_player_controller))
  (UserInterface|Viewport|AddtoViewport _returnvalue 0)
  (bind _newvalue (Ability|Tasks|WaitForAttributeChanged 0 "(AttributeName=\"MaxHealth\",Attribute=/Script/LDJam55.CharacterAttributeSet:MaxHealth,AttributeOwner=\"/Script/CoreUObject.Class'/Script/LDJam55.CharacterAttributeSet'\")")
    (:then
      (bind _newvalue_2 (Ability|Tasks|WaitForAttributeChanged 0 "(AttributeName=\"Health\",Attribute=/Script/LDJam55.CharacterAttributeSet:Health,AttributeOwner=\"/Script/CoreUObject.Class'/Script/LDJam55.CharacterAttributeSet'\")")
        (:then
          (GameplayAbilities|GiveAbility (Variables|Default|GetAbilitySystem) "/Game/Game/Player/Abilities/GA_SummonCube.GA_SummonCube_C" 0 -1)
          (bind (_asynctaskproxy _attribute _newvalue_3 _oldvalue) (Ability|Tasks|WaitForAttributeChanged 0 "(AttributeName=\"ChannelingSpeed\",Attribute=/Script/LDJam55.SummoningAttributeSet:ChannelingSpeed,AttributeOwner=\"/Script/CoreUObject.Class'/Script/LDJam55.SummoningAttributeSet'\")")
            (:then
              (bind (_asynctaskproxy_2 _attribute_2 _newvalue_4 _oldvalue_2) (Ability|Tasks|WaitForAttributeChanged 0 "(AttributeName=\"ChannelingDuration\",Attribute=/Script/LDJam55.SummoningAttributeSet:ChannelingDuration,AttributeOwner=\"/Script/CoreUObject.Class'/Script/LDJam55.SummoningAttributeSet'\")")
                (:Changed
                  (Variables|Default|SetScaleDuration (* (/ (Variables|Default|GetScaleDuration) _oldvalue_2) _newvalue_4)))))
            (:Changed
              (Variables|Default|SetScalePerSecond (* (/ (Variables|Default|GetScalePerSecond) _oldvalue) _newvalue_3))
              (Variables|Default|SetScaleDuration (/ (* _oldvalue (Variables|Default|GetScaleDuration)) _newvalue_3)))))
        (:Changed
          (bind _output_get (Variables|/Game/Game/UI/HUD/WBP_HUD.WBP_HUD_C|SetHealth _returnvalue _newvalue_2))
          (if (<= _output_get 0.0)
            (bind _returnvalue_2 (UserInterface|CreateWidget "/Game/Game/UI/GameOver/WBP_GameOver.WBP_GameOver_C"))
            (UserInterface|Viewport|AddtoViewport _returnvalue_2 0)
            (Actor|DestroyActor)))))
    (:Changed
      (Variables|/Game/Game/UI/HUD/WBP_HUD.WBP_HUD_C|SetMaxHealth _returnvalue _newvalue))))

(event EventTick
  (params (DeltaSeconds :type Float%20%28single-precision%29))
  (bind _returnvalue (Transformation|GetActorLocation))
  (bind _returnvalue_2 (Utilities|Time|GetWorldDeltaSeconds))
  (bind _scalepersecond (Variables|Default|GetScalePerSecond))
  (bind _springarm (Variables|Default|GetSpringArm))
  (bind _summonedcube (Variables|Default|GetSummonedCube))
  (bind _returnvalue_3 (Transformation|GetActorScale3D _summonedcube))
  (bind _returnvalue_4 (* _returnvalue_2 _scalepersecond))
  (bind _returnvalue_5 (+ _returnvalue_3 _returnvalue_4))
  (Utilities|FlowControl|Sequence
    (:then_0
      ;[1 1 1] movement
      (bind _asplayer_controller (Utilities|Casting|CastToPlayerController (Pawn|GetController)))
      (if (.ReturnValue (Class|PlayerController|GetHitResultUnderCursorforObjects _asplayer_controller (Utilities|Array|MakeArray "ObjectTypeQuery1") true))
        (Variables|Default|SetTargetLocation (.location (.HitResult (Class|PlayerController|GetHitResultUnderCursorforObjects _asplayer_controller (Utilities|Array|MakeArray "ObjectTypeQuery1") true))))
        (Pawn|SetControlRotation _asplayer_controller (Math|Rotator|FindLookatRotation (Math|Vector|MakeVector (.x _returnvalue) (.y _returnvalue) 0.0) (Math|Vector|MakeVector (.X (Math|Vector|BreakVector (.location (.HitResult (Class|PlayerController|GetHitResultUnderCursorforObjects _asplayer_controller (Utilities|Array|MakeArray "ObjectTypeQuery1") true))))) (.Y (Math|Vector|BreakVector (.location (.HitResult (Class|PlayerController|GetHitResultUnderCursorforObjects _asplayer_controller (Utilities|Array|MakeArray "ObjectTypeQuery1") true))))) 0.0)))))
    (:then_1
      ;[1 1 1] Controll summonedCube
      (if (Variables|Default|GetisSummoning)
        (if (< (Variables|Default|GetCurrentChannelingDuration) (Variables|Default|GetScaleDuration))
          (Transformation|SetActorScale3D _summonedcube _returnvalue_5)
          (Variables|Default|SetCurrentChannelingDuration (+ (Variables|Default|GetCurrentChannelingDuration) _returnvalue_2)))
        (Transformation|SetActorLocationAndRotation (Variables|Default|GetSummonedCube) (Math|Vector|MakeVector (.x (Variables|Default|GetTargetLocation)) (.y (Variables|Default|GetTargetLocation)) (+ (.z (Variables|Default|GetTargetLocation)) (Variables|Default|GetSummoningHeight) (* (.Z (Math|Vector|BreakVector _returnvalue_5)) 5e+01))) (Pawn|GetControlRotation :!class /Script/Engine.Pawn) false true)
        (Variables|/Script/Engine.SpringArmComponent|SetTargetArmLength (Variables|Default|GetSpringArm) (Math|Float|Max(Float) (* (+ (.z (Variables|Default|GetTargetLocation)) (Variables|Default|GetSummoningHeight) (* (.Z (Math|Vector|BreakVector _returnvalue_5)) 5e+01)) 2.5) 1e+03))
        (else
          (Variables|Default|SetCurrentChannelingDuration 0.0)
          (Variables|/Script/Engine.SpringArmComponent|SetTargetArmLength _springarm (Math|Float|Max(Float) (- (Variables|/Script/Engine.SpringArmComponent|GetTargetArmLength _springarm) (* DeltaSeconds 2e+02)) 1e+03)))))))

(fn ConstructionScript)