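; Basic enemy that runs the BT_BasicEnemy behavior tree and hurts the player on contact.
; On overlap it applies GE_ContactDamage through the Gameplay Ability System and launches the player away horizontally with a fixed upward pop.
; An attribute-change listener broadcasts OnDeath and destroys the actor when the watched value drops from positive to zero or below.
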(event EventBeginPlay
  (bind (_asynctaskproxy _attribute _newvalue _oldvalue) (Ability|Tasks|WaitForAttributeChanged 0 "(AttributeName=\"Health\",Attribute=/Script/LDJam55.CharacterAttributeSet:Health,AttributeOwner=\"/Script/CoreUObject.Class'/Script/LDJam55.CharacterAttributeSet'\")")
    (:then
      (bind _asaicontroller (Utilities|Casting|CastToAIController (Pawn|GetController self)))
      (AI|RunBehaviorTree _asaicontroller "/Game/Game/Enemies/BT_BasicEnemy.BT_BasicEnemy"))
    (:Changed
      (if (and (<= _newvalue 0.0) (> _oldvalue 0.0))
        (Default|CallOnDeath)
        (Actor|DestroyActor)))))

(event EventTick
  (params (DeltaSeconds :type Float%20%28single-precision%29)))

(event Collision|EventActorBeginOverlap
  (params (OtherActor :type Actor%20Object%20Reference))
  (bind _asbp_player_character (Utilities|Casting|CastToBP_PlayerCharacter OtherActor))
  (GameplayEffects|ApplyGameplayEffectToTarget :self (Variables|Default|GetAbilitySystem) :GameplayEffectClass "/Game/Game/Enemies/GE_ContactDamage.GE_ContactDamage_C" :Target (Ability|GetAbilitySystemComponent _asbp_player_character))
  (Utilities|IsValid _asbp_player_character
    (:Is%20Valid
      (Character|LaunchCharacter _asbp_player_character (Math|Vector|MakeVector (.x (* (Math|Vector|Normalize (Math|Vector|MakeVector (.x (- (Transformation|GetActorLocation _asbp_player_character) (Transformation|GetActorLocation))) (.y (- (Transformation|GetActorLocation _asbp_player_character) (Transformation|GetActorLocation))) 0.0)) "300.000000,300.000000,300.000000")) (.y (* (Math|Vector|Normalize (Math|Vector|MakeVector (.x (- (Transformation|GetActorLocation _asbp_player_character) (Transformation|GetActorLocation))) (.y (- (Transformation|GetActorLocation _asbp_player_character) (Transformation|GetActorLocation))) 0.0)) "300.000000,300.000000,300.000000")) 2e+02) true true))))

(fn ConstructionScript)