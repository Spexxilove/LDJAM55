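; Game mode for a survivor-style game that runs enemy spawning, kill combos and level-up progression.
; Tick spawns BP_BasicEnemy on a ring around the player at steadily shrinking intervals, up to a population cap.
; Each enemy's OnDeath feeds OnEnemyKilled, which updates counts and refreshes a timed combo, whose best is saved on expiry.
; Reaching a growing kill threshold opens WBP_UpgradeSelection after a short delay.
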(event Custom|OnEnemyKilled
  (Math|Integer|DecrementInt (Variables|Default|GetNumberOfEnemies)
    (:%20%20
      (Math|Integer|IncrementInt (Variables|Default|GetKilledEnemies)
        (:%20%20
          (Math|Integer|IncrementInt (Variables|Default|GetKIllCombo)
            (:%20%20
              (Variables|Default|SetComboTimer 3.0)
              (Variables|Default|SetIsComboActive true)
              ;[1 1 1] Level Up
              (bind _result (Math|Integer|IncrementInt (Variables|Default|GetKillsSinceLevelUp))
                (:%20%20
                  (if (<= (Variables|Default|GetKillsToLevelUp) _result)
                    (Variables|Default|SetShouldLevelUp true)
                    (Variables|Default|SetLevelUpTimer 1.5)
                    (Variables|Default|SetKillsToLevelUp (Math|Float|Truncate (* (Variables|Default|GetKillsToLevelUp) 1.25)))
                    (Variables|Default|SetKillsSinceLevelUp 0)))))))))))

(event EventBeginPlay)

(event EventTick
  (params (DeltaSeconds :type Float%20%28single-precision%29))
  (bind _returnvalue (Math|Random|RandomUnitVector))
  (bind _returnvalue_2 (Class|KismetMathLibrary|VectorNormal2D _returnvalue 0.0001))
  (Utilities|FlowControl|Sequence
    (:then_0
      (if (and (> (+ (Variables|Default|GetTimeSinceLastSpawn) DeltaSeconds) (Variables|Default|GetTimeToNextSpawn)) (< (Variables|Default|GetNumberOfEnemies) 50))
        (bind _returnvalue_3 (Game|SpawnActorfromClass "/Game/Game/Enemies/BP_BasicEnemy.BP_BasicEnemy_C" (Math|Transform|MakeTransform (+ (* _returnvalue_2 "2000.000000,2000.000000,0.000000") (Transformation|GetActorLocation (Game|Player|GetPlayerPawn 0))) (Math|Rotator|MakeRotfromZ _returnvalue_2) "1.000000,1.000000,1.000000") "Undefined" "MultiplyWithRoot" 0 0))
        (EventDispatchers|BindEventtoOnDeath _returnvalue_3 (delegate Custom|OnEnemyKilled))
        (Variables|Default|SetTimeSinceLastSpawn 0.0)
        (Variables|Default|SetTimeToNextSpawn (* (Variables|Default|GetTimeToNextSpawn) 0.975))
        (Math|Integer|IncrementInt (Variables|Default|GetNumberOfEnemies))
        (else
          (Variables|Default|SetTimeSinceLastSpawn (+ (Variables|Default|GetTimeSinceLastSpawn) DeltaSeconds)))))
    (:then_1
      (if (Variables|Default|GetIsComboActive)
        (if (<= (- (Variables|Default|GetComboTimer) DeltaSeconds) 0.0)
          (Variables|Default|SetIsComboActive false)
          (Variables|Default|SetHighestCombo (Math|Integer|Max(Integer) (Variables|Default|GetKIllCombo) (Variables|Default|GetHighestCombo)))
          (Variables|Default|SetKIllCombo 0)
          (else
            (Variables|Default|SetComboTimer (- (Variables|Default|GetComboTimer) DeltaSeconds))))))
    (:then_2
      (if (Variables|Default|GetShouldLevelUp)
        (bind _output_get (Variables|Default|SetLevelUpTimer (- (Variables|Default|GetLevelUpTimer) DeltaSeconds)))
        (if (<= _output_get 0.0)
          (Variables|Default|SetShouldLevelUp false)
          (bind _returnvalue_4 (UserInterface|CreateWidget "/Game/Game/UI/UpgradeSelection/WBP_UpgradeSelection.WBP_UpgradeSelection_C"))
          (UserInterface|Viewport|AddtoViewport _returnvalue_4 0))))))

(fn ConstructionScript)